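; Game mode for the 2D ruled mode that broadcasts the active rule through SetNewRule and runs a repeating siren warning.
; BeginPlay sets the starting rule with a door sound and creates the WB_Siren widget.
; An endless delay-driven loop then periodically plays an alarm and blinks the siren on screen, without changing the rule itself.
; Rule changes arrive through PushNextRule, which rebroadcasts the given rule and replays the door sound.
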(event `self.ReceiveBeginPlay`
  (bind _sirenwidget (`self.SirenWidget`))
  (`KismetSystemLibrary.Delay` 0.2)
  (bind _returnvalue (`|CreateWidget` "/Game/Luke/HUD_UI_Luke/WB_Siren.WB_Siren_C"))
  (set `self.SirenWidget` _returnvalue)
  (bind _output_get (set `self.starting rule` 0))
  (`self.Set New Rule` _output_get)
  (`GameplayStatics.PlaySound2D` "/Game/Chaz/Sound/322875__thedonkey__sci-fi-door.322875__thedonkey__sci-fi-door" 1.0 1.0 0.0 null null)
  (`KismetSystemLibrary.Delay` 5.0 :!label _label)
  (`GameplayStatics.PlaySound2D` "/Game/Chaz/Sound/33729__jobro__1-alarm-short-b.33729__jobro__1-alarm-short-b" 1.0 1.0 0.0 null null)
  (if (>= (`self.Looped`) 4) :!label _label_2
    (set `self.Looped` 0)
    (goto _label)
    (else
      (`/Engine/EditorBlueprintResources/StandardMacros.IncrementInt` (`self.Looped`)
        (:`  `
          (`KismetSystemLibrary.Delay` 0.2)
          (`UserWidget.AddToViewport` _sirenwidget 0)
          (`KismetSystemLibrary.Delay` 0.2)
          (`Widget.RemoveFromParent` _sirenwidget)
          (goto _label_2))))))

(event `/Game/Luke/Rule_Interface.Push_Next_Rule`
  (params (NextRule :type Integer))
  (`self.Set New Rule` NextRule)
  (`GameplayStatics.PlaySound2D` "/Game/Chaz/Sound/322875__thedonkey__sci-fi-door.322875__thedonkey__sci-fi-door" 1.0 1.0 0.0 null null))

(fn `UserConstructionScript`)