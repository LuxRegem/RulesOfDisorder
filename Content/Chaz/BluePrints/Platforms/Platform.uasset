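; Platform actor that reacts to gravity and collision rule changes broadcast by BP_2d_Ruled_GameMode.
; SetNewRule toggles mesh gravity, adding an upward force for reversed gravity, switches the collision component's constraint mode and swaps the mesh's collision object type.
; Under reversed gravity, player overlaps send surface messages: found after a short delay if the collision rule is 0, lost on exit.
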(event `self.ReceiveBeginPlay`
  (add `/Game/Playar/Blueprints/BP_2d_Ruled_GameMode.Set New Rule` (cast `/Game/Playar/Blueprints/BP_2d_Ruled_GameMode` (`GameplayStatics.GetGameMode`) :!pure true) (delegate `Set New Rule`)))

(event `Set New Rule`
  (params (`New Grav Rule` :type Integer) (`New Colision Rule` :type Integer))
  (bind _staticmesh1 (`self.StaticMesh1`))
  (bind _staticmesh1_2 (`self.StaticMesh1`))
  (bind _copllison (`self.Copllison`))
  (set `self.Current Grav Rule` `New Grav Rule`)
  (set `self.Current Collision Rule` `New Colision Rule`)
  (`|ExecutionSequence`
    (:`then_0`
      (if (== (`self.Current Grav Rule`) 1)
        ;[1 0 0.7989] Reverse Gravity Rule
        (`PrimitiveComponent.SetEnableGravity` _staticmesh1_2 false)
        (`PrimitiveComponent.AddForce` _staticmesh1_2 (0.0 0.0 20000.0) "None" true)
        (`PrimitiveComponent.SetConstraintMode` _copllison "Default")))
    (:`then_1`
      (if (== (`self.Current Grav Rule`) 0)
        (`PrimitiveComponent.SetEnableGravity` _staticmesh1_2 true)
        (`PrimitiveComponent.SetConstraintMode` _copllison "None")))
    (:`then_2`
      (if (== (`self.Current Collision Rule`) 0)
        ;[1 0 0.7989] Invert Collision Rule
        (`PrimitiveComponent.SetCollisionObjectType` _staticmesh1 "ECC_GameTraceChannel5")))
    (:`then_3`
      (if (== (`self.Current Collision Rule`) 1)
        (`PrimitiveComponent.SetCollisionObjectType` _staticmesh1 "ECC_GameTraceChannel2")))))

(event `self.ReceiveActorBeginOverlap`
  (params (OtherActor :type "Actor Object Reference"))
  ;[1 1 1] Surface
  (if (== OtherActor (`GameplayStatics.GetPlayerPawn` 0))
    (if (== (`self.Current Collision Rule`) 0)
      (if (== (`self.Current Grav Rule`) 1)
        (`KismetSystemLibrary.Delay` 0.374)
        (message `/Game/Luke/Rule_Interface.FoundSurface` OtherActor)))))

(event `self.ReceiveActorEndOverlap`
  (params (OtherActor :type "Actor Object Reference"))
  ;[1 1 1] Surface
  (if (== OtherActor (`GameplayStatics.GetPlayerPawn` 0))
    (if (== (`self.Current Grav Rule`) 1)
      (message `/Game/Luke/Rule_Interface.LostSurface` OtherActor))))

(fn `UserConstructionScript`)