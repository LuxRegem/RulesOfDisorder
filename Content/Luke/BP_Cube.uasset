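; BP_Cube is a physics cube that responds to gravity and collision rule changes from BP_2d_Ruled_GameMode.
; SetNewRule, bound on BeginPlay, toggles reverse gravity and switches the mesh's collision object type between two custom channels.
; Reversed gravity disables normal gravity, applies an upward kick and sustains upward acceleration on Tick.
; Player overlaps send found-surface messages under reverse gravity with collision rule 1, and lost-surface messages under reverse gravity alone.
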(event `self.ReceiveBeginPlay`
  (add `/Game/Playar/Blueprints/BP_2d_Ruled_GameMode.Set New Rule` (cast `/Game/Playar/Blueprints/BP_2d_Ruled_GameMode` (`GameplayStatics.GetGameMode`) :!pure true) (delegate `Set New Rule`)))

(event `self.ReceiveTick`
  (params (DeltaSeconds :type "Float (single-precision)"))
  (if (`self.Reverse Gravity`)
    (`PrimitiveComponent.AddForce` (`self.StaticMesh`) (0.0 0.0 2000.0) "None" true)))

(event `Set New Rule`
  (params (`New Grav Rule` :type Integer) (`New Colision Rule` :type Integer))
  (bind _staticmesh (`self.StaticMesh`))
  (bind _staticmesh_2 (`self.StaticMesh`))
  (set `self.Current Grav Rule` `New Grav Rule`)
  (set `self.Current Collision Rule` `New Colision Rule`)
  (`|ExecutionSequence`
    (:`then_0`
      (if (== (`self.Current Grav Rule`) 1)
        ;[1 0 0.7989] Reverse Gravity Rule
        (`PrimitiveComponent.SetEnableGravity` _staticmesh false)
        (`PrimitiveComponent.AddForce` _staticmesh (0.0 0.0 20000.0) "None" true)
        (set `self.Reverse Gravity` true)))
    (:`then_1`
      (if (== (`self.Current Grav Rule`) 0)
        (`PrimitiveComponent.SetEnableGravity` _staticmesh true)
        (set `self.Reverse Gravity` false)))
    (:`then_2`
      (if (== (`self.Current Collision Rule`) 0)
        ;[1 0 0.7989] Invert Collision Rule
        (`PrimitiveComponent.SetCollisionObjectType` _staticmesh_2 "ECC_GameTraceChannel2")))
    (:`then_3`
      (if (== (`self.Current Collision Rule`) 1)
        (`PrimitiveComponent.SetCollisionObjectType` _staticmesh_2 "ECC_GameTraceChannel5")))))

(event `self.ReceiveActorBeginOverlap`
  (params (OtherActor :type "Actor Object Reference"))
  ;[1 1 1] Surface
  (if (== OtherActor (`GameplayStatics.GetPlayerPawn` 0))
    (if (== (`self.Current Collision Rule`) 1)
      (if (== (`self.Current Grav Rule`) 1)
        (`KismetSystemLibrary.Delay` 0.0)
        (message `/Game/Luke/Rule_Interface.FoundSurface` OtherActor)))))

(event `self.ReceiveActorEndOverlap`
  (params (OtherActor :type "Actor Object Reference"))
  ;[1 1 1] Surface
  (if (== OtherActor (`GameplayStatics.GetPlayerPawn` 0))
    (if (== (`self.Current Grav Rule`) 1)
      (message `/Game/Luke/Rule_Interface.LostSurface` OtherActor))))

(fn `UserConstructionScript`)