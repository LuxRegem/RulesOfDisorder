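; BP_Surface_Overlap is an overlap actor that tells the player pawn when it finds or loses a surface.
; On BeginPlay it binds to BP_2d_Ruled_GameMode to keep its current rule updated.
; When the player enters under rule 1, it sends FoundSurfaceMessage to the pawn after a short delay.
; Exit sends LostSurfaceMessage immediately, whatever the rule, and does not cancel a pending found message.
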(event `self.ReceiveBeginPlay`
  ;[1 1 1] Set Current Rule
  (add `/Game/Playar/Blueprints/BP_2d_Ruled_GameMode.Set New Rule` (cast `/Game/Playar/Blueprints/BP_2d_Ruled_GameMode` (`GameplayStatics.GetGameMode`) :!pure true) (delegate `Set New Rule`)))

(event `Set New Rule`
  (params (`New Rule` :type Integer))
  ;[1 1 1] Set Current Rule
  (set `self.Current Rule` `New Rule`))

(event `self.ReceiveActorBeginOverlap`
  (params (OtherActor :type "Actor Object Reference"))
  ;[1 1 1] Surface
  (if (== OtherActor (`GameplayStatics.GetPlayerPawn` 0))
    (if (== (`self.Current Rule`) 1)
      (`KismetSystemLibrary.Delay` 0.374)
      (message `/Game/Luke/Rule_Interface.FoundSurface` OtherActor))))

(event `self.ReceiveActorEndOverlap`
  (params (OtherActor :type "Actor Object Reference"))
  ;[1 1 1] Surface
  (if (== OtherActor (`GameplayStatics.GetPlayerPawn` 0))
    (message `/Game/Luke/Rule_Interface.LostSurface` OtherActor)))

(fn `UserConstructionScript`)